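; BP_Door is an interactable door that swings away from either side in stages: closed, partially opened, open, then closed again.
; Interaction picks the swing sign from a dot product of player and door forward vectors, then a timer ends motion and advances the state.
; While interacting, Tick interpolates yaw toward the state's target.
; An end-overlap event attempts auto-close after a facing check, without changing the state.
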(event OnComponentEndOverlap(BoxCollision)
  (params (OverlappedComponent :type Primitive%20Component%20Object%20Reference) (OtherActor :type Actor%20Object%20Reference) (OtherComp :type Primitive%20Component%20Object%20Reference) (OtherBodyIndex :type Integer))
  (bind _returnvalue (Game|GetPlayerCharacter 0))
  (bind _returnvalue_2 (Transformation|GetActorForwardVector _returnvalue))
  ;[0.4375 0.291 0] Automatic Door Closed
  (if (and (== OtherActor _returnvalue) (Math|Boolean|NORBoolean (>= (.y _returnvalue_2) 0.7) (<= (.y _returnvalue_2) -7.0)))
    (Utilities|FlowControl|Delay 0.5)
    (Variables|Default|SetbIsInteractingWithDoor? true)
    (CallFunction|HandleRotation 0.0)
    (Utilities|FlowControl|Delay 1.4)
    (Variables|Default|SetbIsInteractingWithDoor? false)))

(event Custom|HandleRotation
  (params (Set%20Rotation :type Float%20%28double-precision%29))
  ;[0.5104 0.3023 0] Handle Rotation
  (Transformation|SetRelativeRotation (Variables|Default|GetDoor) (Math|Rotator|MakeRotator 0.0 0.0 (Math|Interpolation|FInterpTo (.Yaw (Math|Rotator|BreakRotator (Variables|/Script/Engine.SceneComponent|GetRelativeRotation (Variables|Default|GetDoor)))) Set%20Rotation (Utilities|Time|GetWorldDeltaSeconds) (Variables|Default|GetInterp%20Speed))) false false))

(event Custom|HandleDoor
  ;[0.6719 0.4242 0.02239] Handle Door (Rotasi Pintu tergantung dari Door Statenya)
  (switch Utilities|FlowControl|Switch|SwitchonE_DoorStates (Variables|Default|GetEDoorStates)
    (:NewEnumerator0
      (CallFunction|HandleRotation (* 15.0 (Variables|Default|GetDoor%20Open%20Side))))
    (:NewEnumerator1
      (CallFunction|HandleRotation (* (Variables|Default|GetDoor%20Open%20Angle) (Variables|Default|GetDoor%20Open%20Side))))
    (:NewEnumerator2
      (CallFunction|HandleRotation 0.0))))

(event Custom|isInteractingWithDoor
  (params (Player :type BP%20First%20Person%20Character%20Object%20Reference))
  ;[0.4375 0.291 0] Door Interaction Math
  (if (> (Math|Vector|DotProduct (Transformation|GetActorForwardVector Player) (Math|Vector|GetForwardVector (Variables|Default|GetDoorOpenLocation))) 0.0)
    (Variables|Default|SetDoor%20Open%20Side 1.0)
    (else
      (Variables|Default|SetDoor%20Open%20Side -1.0)))
  (Variables|Default|SetbIsInteractingWithDoor? true)
  (Utilities|Time|SetTimerbyEvent (delegate Custom|CustomEvent) (Variables|Default|GetDoor%20Sound%20Time)))

(event Custom|CustomEvent
  ;[0.4375 0.291 0] Door Interaction Math
  (Variables|Default|SetbIsInteractingWithDoor? false)
  (switch Utilities|FlowControl|Switch|SwitchonE_DoorStates (Variables|Default|GetEDoorStates)
    (:NewEnumerator0
      (Variables|Default|SetEDoorStates "NewEnumerator1"))
    (:NewEnumerator1
      (Variables|Default|SetEDoorStates "NewEnumerator2"))
    (:NewEnumerator2
      (Variables|Default|SetEDoorStates "NewEnumerator0"))))

(event EventBeginPlay
  (bind _asbp_first_person_character (Utilities|Casting|CastToBP_FirstPersonCharacter (Game|GetPlayerCharacter 0)))
  (Variables|Default|SetCharacter%20Ref _asbp_first_person_character))

(event EventTick
  (params (DeltaSeconds :type Float%20%28single-precision%29))
  (if (Variables|Default|GetbIsInteractingWithDoor?)
    (CallFunction|HandleDoor)))

(fn ConstructionScript)